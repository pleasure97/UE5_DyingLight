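; Enemy AI character that performs the mutant's parkour and attack moves using data from its EnemyController.
; Ledge climbs, block jumps and jump attacks set Motion Warping targets and fly during montages; drop-downs face the target, and swipes alternate hands.
; Completed moves set success flags and call the controller's UpdateState; chase events toggle FollowEnemy.
; Jump attack draws debug spheres and has no montage assigned.
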(event Custom|BP_AI_ParkourLedge
  (bind _returnvalue (Transformation|GetActorLocation))
  (bind _returnvalue_2 (Transformation|GetActorForwardVector))
  (bind _returnvalue_3 (Transformation|GetActorLocation))
  (bind _returnvalue_4 (Transformation|GetActorRotation))
  (bind _as_enemy_controller (Variables|Default|GetAs%20Enemy%20Controller))
  (bind _as_enemy_controller_2 (Variables|Default|GetAs%20Enemy%20Controller))
  (bind _returnvalue_5 (* _returnvalue_2 48.0))
  (bind _referenceparkourtargetvector (Variables|/Game/AI_Volatile/AI/EnemyController.EnemyController_C|GetReferenceParkourTargetVector _as_enemy_controller))
  (bind (_x _y) (Math|Vector|BreakVector _referenceparkourtargetvector))
  (bind _returnvalue_6 (+ _returnvalue _returnvalue_5))
  (bind (_x_2 _y_2) (Math|Vector|BreakVector _returnvalue_6))
  (if (not (Variables|/Game/AI_Volatile/AI/EnemyController.EnemyController_C|GetbHillDown _as_enemy_controller_2))
    (Pawn|Components|CharacterMovement|SetMovementMode (Variables|Character|GetCharacterMovement) "MOVE_Flying" 0)
    (Collision|SetActorEnableCollision false)
    (Class|MotionWarpingComponent|AddorUpdateWarpTarget (Variables|Default|GetMotionWarping) (Utilities|Struct|MakeMotionWarpingTarget "Ledge Climb" (Math|Vector|MakeVector _x_2 _y_2 (- (.Z (Math|Vector|BreakVector _referenceparkourtargetvector)) 115.0)) _returnvalue_4 0 "None" false))
    (Class|MotionWarpingComponent|AddorUpdateWarpTarget (Variables|Default|GetMotionWarping) (Utilities|Struct|MakeMotionWarpingTarget "Ledge Climb Forward" _referenceparkourtargetvector _returnvalue_4 0 "None" false))
    (Animation|Montage|PlayMontage (Variables|Character|GetMesh) "/Game/AI_Volatile/Vol/AIAnimation/MantleLedge_Montage.MantleLedge_Montage"
      (:OnCompleted
        (Collision|SetActorEnableCollision true)
        (Pawn|Components|CharacterMovement|SetMovementMode (Variables|Character|GetCharacterMovement) "MOVE_Walking" 0)))
    (else
      (Variables|/Game/AI_Volatile/AI/EnemyController.EnemyController_C|SetbHillDown _as_enemy_controller_2 false)
      (Transformation|SetActorRotation (Math|Rotator|FindLookatRotation (Math|Vector|MakeVector (.x _returnvalue_3) (.y _returnvalue_3) 0.0) (Math|Vector|MakeVector _x _y 0.0)))
      (Animation|Montage|PlayMontage (Variables|Character|GetMesh) "/Game/AI_Volatile/Vol/AIAnimation/Mutant_Jump_Down_Montage.Mutant_Jump_Down_Montage"
        (:OnCompleted
          _))))
  (Variables|Default|SetSuccess true)
  (Default|UpdateState (Variables|Default|GetAs%20Enemy%20Controller)))

(event Custom|StopChasingPlayer
  (Variables|Default|SetFollow%20Enemy false)
  (Components|Movement|StopMovementImmediately (Variables|Character|GetCharacterMovement)))

(event Custom|Start_ChasingPlayer
  (Variables|Default|SetFollow%20Enemy true))

(event Custom|Play%20JumpAttack
  (bind _as_enemy_controller (Variables|Default|GetAs%20Enemy%20Controller))
  (bind _jumpattackmiddle (Variables|/Game/AI_Volatile/AI/EnemyController.EnemyController_C|GetJumpAttackMiddle _as_enemy_controller))
  (bind _jumpattackend (Variables|/Game/AI_Volatile/AI/EnemyController.EnemyController_C|GetJumpAttackEnd _as_enemy_controller))
  (bind _targetlook (Variables|/Game/AI_Volatile/AI/EnemyController.EnemyController_C|GetTargetLook _as_enemy_controller))
  (Rendering|Debug|DrawDebugSphere _jumpattackmiddle 3e+01 12 "(R=1.000000,G=0.000000,B=0.095971,A=1.000000)" 15.0 1e+01)
  (Rendering|Debug|DrawDebugSphere _jumpattackend 3e+01 12 "(R=0.000000,G=1.000000,B=0.213290,A=1.000000)" 15.0 1e+01)
  (Pawn|Components|CharacterMovement|SetMovementMode (Variables|Character|GetCharacterMovement) "MOVE_Flying" 0)
  (Class|MotionWarpingComponent|AddorUpdateWarpTarget (Variables|Default|GetMotionWarping) (Utilities|Struct|MakeMotionWarpingTarget "Middle" _jumpattackmiddle _targetlook 0 "None" false))
  (Class|MotionWarpingComponent|AddorUpdateWarpTarget (Variables|Default|GetMotionWarping) (Utilities|Struct|MakeMotionWarpingTarget "End" _jumpattackend _targetlook 0 "None" false))
  (Animation|Montage|PlayMontage (Variables|Character|GetMesh) 0
    (:OnCompleted
      (Variables|Default|SetJump%20Attack%20Success true)
      (Pawn|Components|CharacterMovement|SetMovementMode (Variables|Character|GetCharacterMovement) "MOVE_Walking" 0)
      (Default|UpdateState (Variables|Default|GetAs%20Enemy%20Controller)))))

(event Custom|JumpNextBlock
  (bind _returnvalue (Transformation|GetActorRotation))
  (bind _as_enemy_controller (Variables|Default|GetAs%20Enemy%20Controller))
  (bind _referenceparkourtargetvector (Variables|/Game/AI_Volatile/AI/EnemyController.EnemyController_C|GetReferenceParkourTargetVector _as_enemy_controller))
  (bind _jumpstartlocation (Variables|/Game/AI_Volatile/AI/EnemyController.EnemyController_C|GetJumpStartLocation _as_enemy_controller))
  (Pawn|Components|CharacterMovement|SetMovementMode (Variables|Character|GetCharacterMovement) "MOVE_Flying" 0)
  (Collision|SetActorEnableCollision false)
  (Class|MotionWarpingComponent|AddorUpdateWarpTarget (Variables|Default|GetMotionWarping) (Utilities|Struct|MakeMotionWarpingTarget "GO" _jumpstartlocation _returnvalue 0 "None" false))
  (Class|MotionWarpingComponent|AddorUpdateWarpTarget (Variables|Default|GetMotionWarping) (Utilities|Struct|MakeMotionWarpingTarget "Mid" (+ _jumpstartlocation (+ (/ (Math|Vector|VectorLength (- _referenceparkourtargetvector _jumpstartlocation)) 2.0) "0.000000,0.000000,500.000000")) _returnvalue 0 "None" false))
  (Class|MotionWarpingComponent|AddorUpdateWarpTarget (Variables|Default|GetMotionWarping) (Utilities|Struct|MakeMotionWarpingTarget "End" _referenceparkourtargetvector _returnvalue 0 "None" false))
  (Animation|Montage|PlayMontage (Variables|Character|GetMesh) "/Game/AI_Volatile/Vol/AIAnimation/Mutant_Jump_Next_Block.Mutant_Jump_Next_Block"
    (:OnCompleted
      (Collision|SetActorEnableCollision true)
      (Pawn|Components|CharacterMovement|SetMovementMode (Variables|Character|GetCharacterMovement) "MOVE_Walking" 0)
      (Variables|/Game/AI_Volatile/AI/EnemyController.EnemyController_C|SetbCanJumpNextHill (Variables|Default|GetAs%20Enemy%20Controller) false)
      (Variables|Default|SetSuccess true)
      (Default|UpdateState (Variables|Default|GetAs%20Enemy%20Controller)))))

(event Custom|Attack
  (if (and (Variables|Default|GetbAttackHookPoseSelector) (not (Variables|Default|GetSuccess)))
    (Variables|Default|SetbAttackHookPoseSelector false)
    (Animation|Montage|PlayMontage (Variables|Character|GetMesh) "/Game/AI_Volatile/Vol/AIAnimation/Mutant_Swiping_Right_Anim_Montage.Mutant_Swiping_Right_Anim_Montage" 1.4
      (:OnCompleted
        _))
    (else
      (Variables|Default|SetbAttackHookPoseSelector true)
      (Animation|Montage|PlayMontage (Variables|Character|GetMesh) "/Game/AI_Volatile/Vol/AIAnimation/Mutant_Swiping_Left_Anim_Montage.Mutant_Swiping_Left_Anim_Montage" 1.4
        (:OnCompleted
          _))))
  (Variables|Default|SetSuccess true)
  (Default|UpdateState (Variables|Default|GetAs%20Enemy%20Controller)))

(event EventBeginPlay)

(event EventPossessed
  (params (NewController :type Controller%20Object%20Reference))
  (bind _asenemy_controller (Utilities|Casting|CastToEnemyController NewController))
  (Variables|Default|SetAs%20Enemy%20Controller _asenemy_controller)
  (bind _outactors (Actor|GetAllActorsOfClass 0)))

(fn ConstructionScript)

(fn Finish
  (params (Success :type Boolean))
  (return Success))