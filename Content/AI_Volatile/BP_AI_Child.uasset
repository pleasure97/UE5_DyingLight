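; Enemy AI character with mutant animations that performs parkour, melee and jump attacks, and bleeds when damaged.
; EnemyController supplies target points for motion-warped montages, switching to Flying during climbs and jumps, and gets UpdateState calls when actions finish.
; AnyDamage feeds Dismemberment, which records broken bones and spawns blood effects and decals.
; Helpers provide ragdoll impulses, knockback and crawl forces; in the second movement state, Tick moves the capsule to the head and leaves blood decals.
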(event Custom|BP_AI_ParkourLedge
  (bind _returnvalue (Transformation|GetActorLocation))
  (bind _returnvalue_2 (Transformation|GetActorForwardVector))
  (bind _returnvalue_3 (Transformation|GetActorLocation))
  (bind _returnvalue_4 (Transformation|GetActorRotation))
  (bind _as_enemy_controller (Variables|Default|GetAs%20Enemy%20Controller))
  (bind _as_enemy_controller_2 (Variables|Default|GetAs%20Enemy%20Controller))
  (bind _returnvalue_5 (* _returnvalue_2 48.0))
  (bind _referenceparkourtargetvector (Variables|/Game/AI_Volatile/AI/EnemyController.EnemyController_C|GetReferenceParkourTargetVector _as_enemy_controller))
  (bind (_x _y) (Math|Vector|BreakVector _referenceparkourtargetvector))
  (bind _returnvalue_6 (+ _returnvalue _returnvalue_5))
  (bind (_x_2 _y_2) (Math|Vector|BreakVector _returnvalue_6))
  (if (not (Variables|/Game/AI_Volatile/AI/EnemyController.EnemyController_C|GetbHillDown _as_enemy_controller_2))
    (Pawn|Components|CharacterMovement|SetMovementMode (Variables|Character|GetCharacterMovement) "MOVE_Flying" 0)
    (Collision|SetActorEnableCollision false)
    (Class|MotionWarpingComponent|AddorUpdateWarpTarget (Variables|Default|GetMotionWarping) (Utilities|Struct|MakeMotionWarpingTarget "Ledge Climb" (Math|Vector|MakeVector _x_2 _y_2 (- (.Z (Math|Vector|BreakVector _referenceparkourtargetvector)) 115.0)) _returnvalue_4 0 "None" false))
    (Class|MotionWarpingComponent|AddorUpdateWarpTarget (Variables|Default|GetMotionWarping) (Utilities|Struct|MakeMotionWarpingTarget "Ledge Climb Forward" _referenceparkourtargetvector _returnvalue_4 0 "None" false))
    (Animation|Montage|PlayMontage (Variables|Character|GetMesh) "/Game/AI_Volatile/Vol/AIAnimation/MantleLedge_Montage.MantleLedge_Montage"
      (:OnCompleted
        (Collision|SetActorEnableCollision true)
        (Pawn|Components|CharacterMovement|SetMovementMode (Variables|Character|GetCharacterMovement) "MOVE_Walking" 0)))
    (else
      (Variables|/Game/AI_Volatile/AI/EnemyController.EnemyController_C|SetbHillDown _as_enemy_controller_2 false)
      (Transformation|SetActorRotation (Math|Rotator|FindLookatRotation (Math|Vector|MakeVector (.x _returnvalue_3) (.y _returnvalue_3) 0.0) (Math|Vector|MakeVector _x _y 0.0)))
      (Animation|Montage|PlayMontage (Variables|Character|GetMesh) "/Game/AI_Volatile/Vol/AIAnimation/Mutant_Jump_Down_Montage.Mutant_Jump_Down_Montage"
        (:OnCompleted
          _))))
  (Variables|Default|SetSuccess true)
  (Default|UpdateState (Variables|Default|GetAs%20Enemy%20Controller)))

(event Custom|StopChasingPlayer
  (Variables|Default|SetFollow%20Enemy false)
  (Components|Movement|StopMovementImmediately (Variables|Character|GetCharacterMovement)))

(event Custom|Start_ChasingPlayer
  (Variables|Default|SetFollow%20Enemy true))

(event Custom|Play%20JumpAttack
  (bind _as_enemy_controller (Variables|Default|GetAs%20Enemy%20Controller))
  (bind _jumpattackmiddle (Variables|/Game/AI_Volatile/AI/EnemyController.EnemyController_C|GetJumpAttackMiddle _as_enemy_controller))
  (bind _jumpattackend (Variables|/Game/AI_Volatile/AI/EnemyController.EnemyController_C|GetJumpAttackEnd _as_enemy_controller))
  (bind _targetlook (Variables|/Game/AI_Volatile/AI/EnemyController.EnemyController_C|GetTargetLook _as_enemy_controller))
  (Rendering|Debug|DrawDebugSphere _jumpattackmiddle 3e+01 12 "(R=1.000000,G=0.000000,B=0.095971,A=1.000000)" 15.0 1e+01)
  (Rendering|Debug|DrawDebugSphere _jumpattackend 3e+01 12 "(R=0.000000,G=1.000000,B=0.213290,A=1.000000)" 15.0 1e+01)
  (Pawn|Components|CharacterMovement|SetMovementMode (Variables|Character|GetCharacterMovement) "MOVE_Flying" 0)
  (Class|MotionWarpingComponent|AddorUpdateWarpTarget (Variables|Default|GetMotionWarping) (Utilities|Struct|MakeMotionWarpingTarget "Middle" _jumpattackmiddle _targetlook 0 "None" false))
  (Class|MotionWarpingComponent|AddorUpdateWarpTarget (Variables|Default|GetMotionWarping) (Utilities|Struct|MakeMotionWarpingTarget "End" _jumpattackend _targetlook 0 "None" false))
  (Animation|Montage|PlayMontage (Variables|Character|GetMesh) 0
    (:OnCompleted
      (Variables|Default|SetJump%20Attack%20Success true)
      (Pawn|Components|CharacterMovement|SetMovementMode (Variables|Character|GetCharacterMovement) "MOVE_Walking" 0)
      (Default|UpdateState (Variables|Default|GetAs%20Enemy%20Controller)))))

(event Custom|JumpNextBlock
  (bind _returnvalue (Transformation|GetActorRotation))
  (bind _as_enemy_controller (Variables|Default|GetAs%20Enemy%20Controller))
  (bind _referenceparkourtargetvector (Variables|/Game/AI_Volatile/AI/EnemyController.EnemyController_C|GetReferenceParkourTargetVector _as_enemy_controller))
  (bind _jumpstartlocation (Variables|/Game/AI_Volatile/AI/EnemyController.EnemyController_C|GetJumpStartLocation _as_enemy_controller))
  (Pawn|Components|CharacterMovement|SetMovementMode (Variables|Character|GetCharacterMovement) "MOVE_Flying" 0)
  (Collision|SetActorEnableCollision false)
  (Class|MotionWarpingComponent|AddorUpdateWarpTarget (Variables|Default|GetMotionWarping) (Utilities|Struct|MakeMotionWarpingTarget "GO" _jumpstartlocation _returnvalue 0 "None" false))
  (Class|MotionWarpingComponent|AddorUpdateWarpTarget (Variables|Default|GetMotionWarping) (Utilities|Struct|MakeMotionWarpingTarget "Mid" (+ _jumpstartlocation (+ (/ (Math|Vector|VectorLength (- _referenceparkourtargetvector _jumpstartlocation)) 2.0) "0.000000,0.000000,500.000000")) _returnvalue 0 "None" false))
  (Class|MotionWarpingComponent|AddorUpdateWarpTarget (Variables|Default|GetMotionWarping) (Utilities|Struct|MakeMotionWarpingTarget "End" _referenceparkourtargetvector _returnvalue 0 "None" false))
  (Animation|Montage|PlayMontage (Variables|Character|GetMesh) "/Game/AI_Volatile/Vol/AIAnimation/Mutant_Jump_Next_Block.Mutant_Jump_Next_Block"
    (:OnCompleted
      (Collision|SetActorEnableCollision true)
      (Pawn|Components|CharacterMovement|SetMovementMode (Variables|Character|GetCharacterMovement) "MOVE_Walking" 0)
      (Variables|/Game/AI_Volatile/AI/EnemyController.EnemyController_C|SetbCanJumpNextHill (Variables|Default|GetAs%20Enemy%20Controller) false)
      (Variables|Default|SetSuccess true)
      (Default|UpdateState (Variables|Default|GetAs%20Enemy%20Controller)))))

(event Custom|Attack
  (if (and (Variables|Default|GetbAttackHookPoseSelector) (not (Variables|Default|GetSuccess)))
    (Variables|Default|SetbAttackHookPoseSelector false)
    (Animation|Montage|PlayMontage (Variables|Character|GetMesh) "/Game/AI_Volatile/Vol/AIAnimation/Mutant_Swiping_Right_Anim_Montage.Mutant_Swiping_Right_Anim_Montage" 1.4
      (:OnCompleted
        _))
    (else
      (Variables|Default|SetbAttackHookPoseSelector true)
      (Animation|Montage|PlayMontage (Variables|Character|GetMesh) "/Game/AI_Volatile/Vol/AIAnimation/Mutant_Swiping_Left_Anim_Montage.Mutant_Swiping_Left_Anim_Montage" 1.4
        (:OnCompleted
          _))))
  (Variables|Default|SetSuccess true)
  (Default|UpdateState (Variables|Default|GetAs%20Enemy%20Controller)))

(event EventBeginPlay)

(event EventTick
  (params (DeltaSeconds :type Float%20%28single-precision%29))
  (bind _mesh (Variables|Character|GetMesh))
  (bind _hit_bone_name (Variables|Combat|GetHit%20Bone%20Name))
  (bind _returnvalue (Transformation|GetSocketLocation _mesh _hit_bone_name))
  (if (Utilities|Enum|Equal(Enum) (Variables|Combat|GetMovementStates) "NewEnumerator1")
    (Utilities|FlowControl|Sequence
      (:then_0
        (Utilities|FlowControl|DoOnce false
          (:Completed
            (Utilities|FlowControl|Delay 3.0)
            (goto _label Open))))
      (:then_1
        (Utilities|FlowControl|Gate true :!label _label
          (:Exit
            (Combat|SetCapsuleLocation))))
      (:then_2
        (Utilities|FlowControl|Delay 1.0)
        (bind _outhit (Collision|LineTraceByChannel _returnvalue (+ _returnvalue (Math|Vector|MakeVector 0.0 0.0 -1e+03)) "TraceTypeQuery1" false 0 "None"))
        (Rendering|Decal|SpawnDecalatLocation "/Game/BloodEffect/Decal/22_High_Velocity_Blood_Spatter_sfcsbflp_8K_inst.22_High_Velocity_Blood_Spatter_sfcsbflp_8K_inst" "-31.500000,-64.000000,-64.000000" (.Location (Collision|BreakHitResult _outhit)) (Math|Conversions|RotationFromXVector (.Normal (Collision|BreakHitResult _outhit))) 6e+01)))))

(event EventPossessed
  (params (NewController :type Controller%20Object%20Reference))
  (bind _asenemy_controller (Utilities|Casting|CastToEnemyController NewController))
  (Variables|Default|SetAs%20Enemy%20Controller _asenemy_controller)
  (bind _outactors (Actor|GetAllActorsOfClass 0)))

(fn ConstructionScript)

(fn Finish
  (params (Success :type Boolean))
  (return Success))

(fn AddForcetoBones
  (Physics|AddForce (Variables|Character|GetMesh) (Utilities|CalculcateCrawlForce 5e+02 3e+03) "head" true)
  (Utilities|FindBrokenBones (Utilities|Array|MakeArray "upperarm_r" "lowerarm_r" "hand_r")
    (:False
      (Physics|AddForce (Variables|Character|GetMesh) (Utilities|CalculcateCrawlForce 1e+03 1e+03) "hand_r" true)
      (Utilities|FindBrokenBones (Utilities|Array|MakeArray "upperarm_l" "lowerarm_l" "hand_l")
        (:False
          (Physics|AddForce (Variables|Character|GetMesh) (Utilities|CalculcateCrawlForce 1e+03 1e+03) "hand_l" true))))))

(fn AnyDamage
  (params (AppliedDamage :type Integer) (HitBoneName :type Name) (DamageCauser :type Actor%20Object%20Reference))
  (Variables|Combat|SetAppliedDamage AppliedDamage)
  (Variables|Combat|SetHit%20Bone%20Name HitBoneName)
  (Variables|Combat|SetDamage%20Causer DamageCauser)
  (Combat|Dismemberment))

(fn RenameBoneName
  (switch name (Variables|Combat|GetHit%20Bone%20Name)
    (:ValveBiped_Bip01_Pelvis_52
      _)
    (:ValveBiped_Bip01_Spine1_50
      _)
    (:ValveBiped_Bip01_Spine2_49
      _)
    (:ValveBiped_Bip01_Neck1_9
      _)
    (:ValveBiped_Bip01_Head1_8
      _))
  (Variables|Combat|SetHit%20Bone%20Name "ValveBiped_Bip01_Spine_51"))

(fn ApplyDamagetoBone
  (bind _breakableboneswithdurablity (Variables|Combat|GetBreakableBonesWithDurablity))
  (bind _hit_bone_name (Variables|Combat|GetHit%20Bone%20Name))
  (bind (_value _returnvalue) (Utilities|Map|Find _breakableboneswithdurablity _hit_bone_name))
  (if _returnvalue
    (Utilities|Map|Add (Variables|Combat|GetBreakableBonesWithDurablity) (Variables|Combat|GetHit%20Bone%20Name) (- _value (Variables|Combat|GetAppliedDamage)))
    (return (<= (.Value (Utilities|Map|Find (Variables|Combat|GetBreakableBonesWithDurablity) (Variables|Combat|GetHit%20Bone%20Name))) 0))))

(fn Dismemberment
  (bind _mesh (Variables|Character|GetMesh))
  (bind _hit_bone_name (Variables|Combat|GetHit%20Bone%20Name))
  (bind _mesh_2 (Variables|Character|GetMesh))
  (bind _returnvalue (Transformation|GetWorldLocation _mesh_2))
  (bind _returnvalue_2 (Transformation|GetSocketTransform _mesh _hit_bone_name "RTS_World"))
  (Niagara|SpawnSystemAttached "/Game/BloodEffect/Niagara/NS_Blood.NS_Blood" _mesh _hit_bone_name (.location _returnvalue_2) (.rotation _returnvalue_2) "KeepWorldPosition" false)
  (Variables|Default|SetHasSplineBroken (== _hit_bone_name "ValveBiped_Bip01_Spine_51"))
  (Utilities|Array|Add (Variables|Combat|GetBrokenBones) (Variables|Combat|GetHit%20Bone%20Name))
  (bind _outhit (Collision|LineTraceByChannel _returnvalue (+ _returnvalue (Math|Vector|MakeVector 0.0 0.0 -1e+03)) "TraceTypeQuery1" false 0 "None"))
  (Rendering|Decal|SpawnDecalatLocation "/Game/BloodEffect/Decal/22_High_Velocity_Blood_Spatter_sfcsbflp_8K_inst.22_High_Velocity_Blood_Spatter_sfcsbflp_8K_inst" "-63.000000,-128.000000,-128.000000" (.Location (Collision|BreakHitResult _outhit)) (Math|Conversions|RotationFromXVector (.Normal (Collision|BreakHitResult _outhit))) 6e+01))

(fn ApplyPhysics
  (bind _mesh (Variables|Character|GetMesh))
  (Physics|SetSimulatePhysics _mesh true)
  (Physics|AddImpulseatLocation _mesh (+ (* (Math|Vector|GetForwardVector (Transformation|GetActorRotation (Game|GetPlayerCameraManager 0))) (Math|Random|RandomFloatinRange 8e+03 1e+04)) (* (Transformation|GetActorUpVector) (Math|Random|RandomFloatinRange 5e+02 8e+03))) (Transformation|GetSocketLocation (Variables|Character|GetMesh) (Variables|Combat|GetHit%20Bone%20Name)) (Variables|Combat|GetHit%20Bone%20Name))
  (Collision|SetCollisionEnabled (Variables|Collision|GetCapsuleComponent) "QueryAndPhysics"))

(fn ChangeMovementType
  (if (Utilities|Enum|Equal(Enum) (Variables|Combat|GetMovementStates) "NewEnumerator0")
    (Variables|Combat|SetMovementStates "NewEnumerator1")))

(fn SetCapsuleLocation
  (Transformation|SetWorldLocation (Variables|Collision|GetCapsuleComponent) (Transformation|GetSocketLocation (Variables|Character|GetMesh) "head") false false))

(fn KnockBack
  (params (DamageCauser :type Actor%20Object%20Reference))
  (bind _returnvalue (Transformation|GetActorLocation DamageCauser))
  (bind _returnvalue_2 (Transformation|GetActorLocation))
  (Character|LaunchCharacter (* (Math|Vector|Normalize (Math|Vector|RotateVectorAroundAxis (Math|Vector|ProjectVectorontoPlane (Math|Vector|GetUnitDirection(Vector) _returnvalue _returnvalue_2) "0.000000,0.000000,1.000000") -25.0 (Math|Vector|GetRightVector (Math|Rotator|FindLookatRotation _returnvalue _returnvalue_2)))) 3e+02) true true))