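; BP_Volatile is an AI enemy that carries out action sequences queued on its BP_AIController.
; PlayAction reads the current action and location, draws debug spheres, and sets blackboard ChaseSelect for climb, jump down, skip, move or scream.
; ForceRest, or an exhausted queue, clears the controller's plan and re-enables Trace.
; StartAttack and DodgeScan overlaps set Attack and Dodge directly; jump-attack logic is present but disconnected.
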(event OnComponentBeginOverlap(DodgeScan)
  (params (OverlappedComponent :type Primitive%20Component%20Object%20Reference) (OtherActor :type Actor%20Object%20Reference) (OtherComp :type Primitive%20Component%20Object%20Reference) (OtherBodyIndex :type Integer) (bFromSweep :type Boolean) (SweepResult :type Hit%20Result%20Structure%20%28by%20ref%29))
  (AI|Components|Blackboard|SetValueasEnum (Variables|/Script/AIModule.AIController|GetBlackboard (Variables|Default|GetAs%20BP%20AIController)) (Utilities|Name|MakeLiteralName "ChaseSelect") (Utilities|Enum|LiteralenumEnum_Action "NewEnumerator7")))

(event OnComponentEndOverlap(JumpAttackScan)
  (params (OverlappedComponent :type Primitive%20Component%20Object%20Reference) (OtherActor :type Actor%20Object%20Reference) (OtherComp :type Primitive%20Component%20Object%20Reference) (OtherBodyIndex :type Integer)))

(event OnComponentBeginOverlap(JumpAttackScan)
  (params (OverlappedComponent :type Primitive%20Component%20Object%20Reference) (OtherActor :type Actor%20Object%20Reference) (OtherComp :type Primitive%20Component%20Object%20Reference) (OtherBodyIndex :type Integer) (bFromSweep :type Boolean) (SweepResult :type Hit%20Result%20Structure%20%28by%20ref%29)))

(event Custom|Play%20Action
  (bind _returnvalue (Transformation|GetActorLocation))
  (bind _as_bp_aicontroller (Variables|Default|GetAs%20BP%20AIController))
  (bind _as_bp_aicontroller_2 (Variables|Default|GetAs%20BP%20AIController))
  (bind _actionlocation (Variables|/Game/AI_Volatile_V3/BP_AIController.BP_AIController_C|GetActionLocation _as_bp_aicontroller))
  (bind _stimulus_location (Variables|/Game/AI_Volatile_V3/BP_AIController.BP_AIController_C|GetStimulus%20Location _as_bp_aicontroller_2))
  (bind _blackboard (Variables|/Script/AIModule.AIController|GetBlackboard _as_bp_aicontroller))
  (bind _actionselect (Variables|/Game/AI_Volatile_V3/BP_AIController.BP_AIController_C|GetActionSelect _as_bp_aicontroller))
  (bind (_x _y) (Math|Vector|BreakVector _stimulus_location))
  (Variables|Default|SetTrace false)
  (if (== (Variables|Default|GetProcessIndex) (Variables|/Game/AI_Volatile_V3/BP_AIController.BP_AIController_C|GetCntMaxActionIndex _as_bp_aicontroller))
    (Utilities|Array|Clear (Variables|/Game/AI_Volatile_V3/BP_AIController.BP_AIController_C|GetTraceVectorArray _as_bp_aicontroller) :!label _label)
    (Utilities|Array|Clear (Variables|/Game/AI_Volatile_V3/BP_AIController.BP_AIController_C|GetIsSkipCheck _as_bp_aicontroller))
    (Utilities|Array|Clear _actionselect)
    (Utilities|Array|Clear _actionlocation)
    (Utilities|Array|Clear (Variables|/Game/AI_Volatile_V3/BP_AIController.BP_AIController_C|GetSkipIndex _as_bp_aicontroller))
    (Variables|/Game/AI_Volatile_V3/BP_AIController.BP_AIController_C|SetSkipCheckIndex _as_bp_aicontroller 0)
    (Variables|/Game/AI_Volatile_V3/BP_AIController.BP_AIController_C|SetCntMaxActionIndex _as_bp_aicontroller 0)
    (Variables|Default|SetProcessIndex 0)
    (Variables|/Game/AI_Volatile_V3/BP_AIController.BP_AIController_C|SetCurrentIndex _as_bp_aicontroller 0)
    (Variables|/Game/AI_Volatile_V3/BP_AIController.BP_AIController_C|SetSkipIndexCnt _as_bp_aicontroller 0)
    (AI|Components|Blackboard|SetValueasEnum _blackboard (Utilities|Name|MakeLiteralName "ChaseSelect") (Utilities|Enum|LiteralenumEnum_Action "NewEnumerator0"))
    (Variables|Default|SetTrace true)
    (elif (and (Utilities|Array|IsNotEmpty _actionlocation) (Utilities|Array|IsNotEmpty _actionselect))
      (Rendering|Debug|DrawDebugSphere (Utilities|Array|Get(acopy) _actionlocation (Variables|Default|GetProcessIndex)) 3e+01 12 "(R=1.000000,G=0.327500,B=0.508953,A=1.000000)" 1e+01 5.0)
      (switch Utilities|FlowControl|Switch|SwitchonEnum_Action (Utilities|Array|Get(acopy) _actionselect (Variables|Default|GetProcessIndex))
        (:NewEnumerator0
          (Math|Integer|IncrementInt (Variables|Default|GetProcessIndex)
            (:%20%20
              (CallFunction|PlayAction))))
        (:NewEnumerator1
          (AI|Components|Blackboard|SetValueasEnum _blackboard (Utilities|Name|MakeLiteralName "ChaseSelect") (Utilities|Enum|LiteralenumEnum_Action "NewEnumerator1")))
        (:NewEnumerator2
          (AI|Components|Blackboard|SetValueasEnum _blackboard (Utilities|Name|MakeLiteralName "ChaseSelect") (Utilities|Enum|LiteralenumEnum_Action "NewEnumerator2")))
        (:NewEnumerator3
          (Rendering|Debug|DrawDebugSphere (Utilities|Array|Get(acopy) _actionlocation (Variables|Default|GetProcessIndex)) 5e+01 12 "(R=0.000000,G=1.000000,B=0.831511,A=1.000000)" 5.0 5.0)
          (AI|Components|Blackboard|SetValueasEnum (Variables|/Script/AIModule.AIController|GetBlackboard (Variables|Default|GetAs%20BP%20AIController)) (Utilities|Name|MakeLiteralName "ChaseSelect") (Utilities|Enum|LiteralenumEnum_Action "NewEnumerator3")))
        (:NewEnumerator4
          (if (Utilities|Operators|NotEqual(!=) :A (Utilities|Array|Get(acopy) _actionlocation (Variables|Default|GetProcessIndex)))
            (AI|Components|Blackboard|SetValueasVector _blackboard (Utilities|Name|MakeLiteralName "TargetLocation") (Utilities|Array|Get(acopy) _actionlocation (Variables|Default|GetProcessIndex)))
            (AI|Components|Blackboard|SetValueasEnum _blackboard (Utilities|Name|MakeLiteralName "ChaseSelect") (Utilities|Enum|LiteralenumEnum_Action "NewEnumerator4"))))
        (:NewEnumerator5
          (Transformation|SetActorRotation (Math|Conversions|RotationFromXVector (Math|Vector|GetRightVector (Math|Rotator|FindLookatRotation (Math|Vector|MakeVector (.x _returnvalue) (.y _returnvalue) 0.0) (Math|Vector|MakeVector _x _y 0.0)))))
          (AI|Components|Blackboard|SetValueasEnum (Variables|/Script/AIModule.AIController|GetBlackboard (Variables|Default|GetAs%20BP%20AIController)) (Utilities|Name|MakeLiteralName "ChaseSelect") (Utilities|Enum|LiteralenumEnum_Action "NewEnumerator5"))))
      (else
        (goto _label)))))

(event Custom|ForceRest
  (bind _as_bp_aicontroller (Variables|Default|GetAs%20BP%20AIController))
  (Utilities|Array|Clear (Variables|/Game/AI_Volatile_V3/BP_AIController.BP_AIController_C|GetTraceVectorArray _as_bp_aicontroller))
  (Utilities|Array|Clear (Variables|/Game/AI_Volatile_V3/BP_AIController.BP_AIController_C|GetIsSkipCheck _as_bp_aicontroller))
  (Utilities|Array|Clear (Variables|/Game/AI_Volatile_V3/BP_AIController.BP_AIController_C|GetActionSelect _as_bp_aicontroller))
  (Utilities|Array|Clear (Variables|/Game/AI_Volatile_V3/BP_AIController.BP_AIController_C|GetActionLocation _as_bp_aicontroller))
  (Utilities|Array|Clear (Variables|/Game/AI_Volatile_V3/BP_AIController.BP_AIController_C|GetSkipIndex _as_bp_aicontroller))
  (Variables|/Game/AI_Volatile_V3/BP_AIController.BP_AIController_C|SetSkipCheckIndex _as_bp_aicontroller 0)
  (Variables|/Game/AI_Volatile_V3/BP_AIController.BP_AIController_C|SetCntMaxActionIndex _as_bp_aicontroller 0)
  (Variables|Default|SetProcessIndex 0)
  (Variables|/Game/AI_Volatile_V3/BP_AIController.BP_AIController_C|SetCurrentIndex _as_bp_aicontroller 0)
  (Variables|/Game/AI_Volatile_V3/BP_AIController.BP_AIController_C|SetSkipIndexCnt _as_bp_aicontroller 0)
  (AI|Components|Blackboard|SetValueasEnum (Variables|/Script/AIModule.AIController|GetBlackboard _as_bp_aicontroller) (Utilities|Name|MakeLiteralName "ChaseSelect") (Utilities|Enum|LiteralenumEnum_Action "NewEnumerator0"))
  (Variables|Default|SetTrace true))

(event Custom|Start%20Attack
  (AI|Components|Blackboard|SetValueasEnum (Variables|/Script/AIModule.AIController|GetBlackboard (Variables|Default|GetAs%20BP%20AIController)) (Utilities|Name|MakeLiteralName "ChaseSelect") (Utilities|Enum|LiteralenumEnum_Action "NewEnumerator6")))

(event EventPossessed
  (params (NewController :type Controller%20Object%20Reference))
  (bind _asbp_aicontroller (Utilities|Casting|CastToBP_AIController NewController))
  (Variables|Default|SetAs%20BP%20AIController _asbp_aicontroller))

(fn ConstructionScript)